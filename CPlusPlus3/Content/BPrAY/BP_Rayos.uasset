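; Lightning ray actor that draws a Niagara beam between points on a set of interactable objects, each given an attached ray-mesh effect at BeginPlay.
; Every Tick it debug-draws each object's closest point to the actor, then, if positions changed, sorts them and feeds the first two into the beam's endpoints.
; A float curve sampled by the distance between those points drives beam width and spawned ray count.
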(event `self.ReceiveBeginPlay`
  (for _array_element (`self.ObjectInteractRay`)
    (`NiagaraFunctionLibrary.SpawnSystemAttached` "/Game/BPrAY/Ns_RayMesh.Ns_RayMesh" (`self.GetComponentByClass` _array_element "/Script/Engine.StaticMeshComponent") "None" (`SceneComponent.K2_GetComponentLocation` (`Actor.RootComponent` _array_element)) (struct) "SnapToTargetIncludingScale")))

(event `self.ReceiveTick`
  (params (DeltaSeconds :type "Float (single-precision)"))
  (bind _returnvalue_location (`KismetMathLibrary.BreakTransform` (`self.GetTransform`)))
  (bind _returnvalue (`KismetMathLibrary.Vector_Distance` (`self.Position1`) (`self.Position0`)))
  (bind _returnvalue_2 (`CurveFloat.GetFloatValue` (`self.CurveBeam`) _returnvalue))
  (`|ExecutionSequence`
    (:`then_0`
      (for _array_element (`self.ObjectInteractRay`)
        (bind _returnvalue_3 (`self.GetClosestPointToPosition` _array_element _returnvalue_location))
        (`KismetSystemLibrary.DrawDebugPoint` _returnvalue_3 13.0 (struct :`R` 1.0 :`B` 0.888188 :`A` 1.0) 0.1))
      (bind _returnvalue_4 (`self.HasSamePosAsPrevious`))
      (if _returnvalue_4
        (`KismetSystemLibrary.PrintString` "igual")
        (`self.ClearArray`)
        (else
          (`|ExecutionSequence`
            (:`then_0`
              ;[0.3037 0.4073 1] Closest Object ,setting Ray
              (`self.UpdatePos`)
              (`self.SortArray`)
              (bind _returnvalue_5 (`self.getPositionByIndex` 0))
              (set `self.Position0` _returnvalue_5)
              (`NiagaraComponent.SetNiagaraVariableVec3` (`self.NS_Ray`) "BeamEnd" _returnvalue_5)
              (bind _returnvalue_6 (`self.getPositionByIndex` 1))
              (bind _output_get (set `self.Position1` _returnvalue_6))
              (`NiagaraComponent.SetNiagaraVariableVec3` (`self.NS_Ray`) "BeamStart" _output_get)
              (`KismetSystemLibrary.PrintText` (`KismetTextLibrary.Conv_DoubleToText` _returnvalue "HalfToEven"))
              (`NiagaraComponent.SetNiagaraVariableFloat` (`self.NS_Ray`) "BeamWidth" (* _returnvalue_2 6.0))
              (`NiagaraComponent.SetVariableInt` (`self.NS_Ray`) "SpawnedRay" (`KismetMathLibrary.FTrunc` (* _returnvalue_2 65.0)))
              (`self.ClearArray`))))))))

(fn `UserConstructionScript`)