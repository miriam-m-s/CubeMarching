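; BP_Ray is an actor that draws a Niagara beam between points on the objects listed in ObjectsInteractRay.
; Each tick it finds each object's closest point to itself, sorts the stored points, sets the first two as beam end and start, then clears the array.
; CurveBeam maps the distance between those points to beam width and spawned ray count.
; Debug points and distance printing remain active.
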(event `self.ReceiveBeginPlay`)

(event `self.ReceiveTick`
  (params (DeltaSeconds :type "Float (single-precision)"))
  (bind _returnvalue_location (`KismetMathLibrary.BreakTransform` (`Actor.GetTransform`)))
  (bind _returnvalue (`KismetMathLibrary.Vector_Distance` (`self.position1`) (`self.postion0`)))
  (bind _returnvalue_2 (`CurveFloat.GetFloatValue` (`self.CurveBeam`) _returnvalue))
  (for _array_element (`self.ObjectsInteractRay`)
    (bind _returnvalue_3 (`self.GetClosestPointToPosition` _array_element _returnvalue_location))
    (`KismetSystemLibrary.DrawDebugPoint` null _returnvalue_3 13.0 (struct :`R` 1.0 :`B` 0.888188 :`A` 1.0) 0.1))
  ;[0.3037 0.4073 1] Closest Object ,setting Ray
  (`self.SortArray`)
  (bind _returnvalue_4 (`self.getPositionByIndex` 0))
  (set `self.postion0` _returnvalue_4)
  (`NiagaraComponent.SetNiagaraVariableVec3` (`self.NS_Ray`) "BeamEnd" _returnvalue_4)
  (bind _returnvalue_5 (`self.getPositionByIndex` 1))
  (set `self.position1` _returnvalue_5)
  (`NiagaraComponent.SetNiagaraVariableVec3` (`self.NS_Ray`) "BeamStart" _returnvalue_5)
  (`KismetSystemLibrary.PrintText` null (`KismetTextLibrary.Conv_DoubleToText` _returnvalue "HalfToEven"))
  (`NiagaraComponent.SetNiagaraVariableFloat` (`self.NS_Ray`) "BeamWidth" (* _returnvalue_2 6.0))
  (`NiagaraComponent.SetVariableInt` (`self.NS_Ray`) "SpawnedRay" (`KismetMathLibrary.FTrunc` (* _returnvalue_2 65.0)))
  (`self.ClearArray`))

(fn `UserConstructionScript`)