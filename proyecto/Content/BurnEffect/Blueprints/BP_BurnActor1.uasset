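; BP_BurnActor1 is a burn effect actor that drives a dissipation fade once its burn finishes.
; On BeginPlay it creates and stores a dynamic instance of RVTWriteMaterial on its mesh, then calls StartBurn, whose logic is not in this graph.
; OnBurnFinished plays a timeline that feeds the material's FinalDissipationAlpha parameter, with debug prints at the start and on each update.
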(event `self.ReceiveBeginPlay`
  (bind _returnvalue (`PrimitiveComponent.CreateDynamicMaterialInstance` (`self.MeshComponent`) 0 (`self.RVTWrite_Material`) "None"))
  (set `self.DynamicMaterialInstance` _returnvalue)
  (`self.StartBurn`))

(event `self.ReceiveTick`
  (params (DeltaSeconds :type "Float (single-precision)")))

(event `self.OnBurnFinished`
  (`KismetSystemLibrary.PrintString` "Hello")
  (bind (_direction _newtrack_0) (`Timeline|Timeline` :!via `PlayFromStart`)
    (:`Update`
      (`KismetSystemLibrary.PrintString` (`KismetStringLibrary.Conv_DoubleToString` _newtrack_0))
      (`MaterialInstanceDynamic.SetScalarParameterValue` (`self.DynamicMaterialInstance`) "FinalDissipationAlpha" _newtrack_0))))

(fn `UserConstructionScript`)