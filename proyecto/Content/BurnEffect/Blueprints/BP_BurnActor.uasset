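; BP_BurnActor is an actor that runs a burn effect on its mesh, drawn through a runtime virtual texture.
; On BeginPlay it creates a dynamic instance of M_BurnRVT on the mesh and calls StartBurn, whose logic lives outside these graphs.
; When OnBurnFinished fires, a timeline drives the material's FinalDissipationAlpha and invalidates the RVT volume's full bounds on every update so the virtual texture re-renders.
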(event `self.ReceiveBeginPlay`
  (bind _returnvalue (`PrimitiveComponent.CreateDynamicMaterialInstance` (`self.MeshComponent`) 0 "/Game/BurnEffect/Materials/M_BurnRVT.M_BurnRVT" "None"))
  (set `self.DMI` _returnvalue)
  (`self.StartBurn`))

(event `self.OnBurnFinished`
  (bind _virtualtexturecomponent (`RuntimeVirtualTextureVolume.VirtualTextureComponent` (`self.RVT_Volume`)))
  (bind (_origin _boxextent _sphereradius) (`KismetSystemLibrary.GetComponentBounds` _virtualtexturecomponent))
  (bind (_direction _newtrack_0) (`Timeline|Timeline`)
    (:`Update`
      (`RuntimeVirtualTextureComponent.Invalidate` _virtualtexturecomponent (`KismetMathLibrary.MakeBoxSphereBounds` _origin _boxextent _sphereradius))
      (`MaterialInstanceDynamic.SetScalarParameterValue` (`self.DMI`) "FinalDissipationAlpha" _newtrack_0))))

(event `self.ReceiveTick`
  (params (DeltaSeconds :type "Float (single-precision)")))

(fn `UserConstructionScript`)